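; Player character Blueprint that turns MoveForward and MoveRight axis input into a movement direction.
; Each axis event adds the scaled actor forward or right vector to DesiredMovement and normalizes the result, with no reset between frames.
; When that vector is non-zero, Tick passes it to CharacterMovement as an input vector, then immediately calls ConsumeInputVector.
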(event EventBeginPlay)

(event Collision|EventActorBeginOverlap
  (params (OtherActor :type Actor%20Object%20Reference)))

(event EventTick
  (params (DeltaSeconds :type Float%20%28single-precision%29))
  (bind _desiredmovement (Variables|Movement|GetDesiredMovement))
  (Utilities|FlowControl|Sequence
    (:then_0
      (if (> (Math|Vector|VectorLength _desiredmovement) 0.0)
        (Class|PawnMovementComponent|AddInputVector (Variables|Character|GetCharacterMovement) _desiredmovement false)
        (Class|PawnMovementComponent|ConsumeInputVector (Variables|Character|GetCharacterMovement))))))

(event Input|AxisEvents|InputAxisMoveForward
  (params (AxisValue :type Float%20%28single-precision%29))
  (Variables|Movement|SetDesiredMovement (Math|Vector|Normalize (+ (* (Transformation|GetActorForwardVector) AxisValue) (Variables|Movement|GetDesiredMovement)))))

(event Input|AxisEvents|InputAxisMoveRight
  (params (AxisValue :type Float%20%28single-precision%29))
  (Variables|Movement|SetDesiredMovement (Math|Vector|Normalize (+ (* (Transformation|GetActorRightVector) AxisValue) (Variables|Movement|GetDesiredMovement)))))

(fn ConstructionScript)